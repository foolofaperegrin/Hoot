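; Owl nest actor holding three chicks that lose satiation over time and perish when it runs out.
; Each chick runs a randomized Delay loop that lengthens with every feeding, while feed events restore satiation and play a chirp.
; Damage rolls randomly to kill a chick or none, and deaths hide the chick and notify UI_Hunger.
; It also registers with the owl and controller, swaps mouse-over visuals and shows a one-time feeding tutorial.
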(event `self.ReceiveBeginPlay`
  (`self.HungerDescreaseChick1`)
  (`self.Chick2HungerDecrease`)
  (`self.Chick3HungerDescrease`)
  (bind _asbp_owl (cast `/Game/Owl/BP_Owl` (`GameplayStatics.GetPlayerPawn` 0)))
  (set `/Game/Owl/BP_Owl.NestObject` self _asbp_owl)
  (bind _ashoot_player_controller (cast `/Game/Owl/Hoot_PlayerController` (`GameplayStatics.GetPlayerController` 0)))
  (set `/Game/Owl/Hoot_PlayerController.NestObject` self _ashoot_player_controller)
  (set `self.SpriteYPosition` (.y (`SceneComponent.K2_GetComponentLocation` (`self.Nest`))))
  (`self.EnableInput` (`GameplayStatics.GetPlayerController` 0))
  (set `self.Chick1Loc` (.location (`SceneComponent.GetRelativeTransform` (`self.Chick1`))))
  (set `self.Chick2Loc` (.location (`SceneComponent.GetRelativeTransform` (`self.Chick2`))))
  (set `self.Chick3Loc` (.location (`SceneComponent.GetRelativeTransform` (`self.Chick3`))))
  (`MovieSceneSequenceExtensions.SetPlaybackStart` "/Game/NewLevelSequence.NewLevelSequence"))

(event `MouseOver`
  (`SceneComponent.SetVisibility` (`self.Nest`) false false)
  (`SceneComponent.SetVisibility` (`self.NestMouseOver`) true false))

(event `MouseOff`
  (`SceneComponent.SetVisibility` (`self.Nest`) true false)
  (`SceneComponent.SetVisibility` (`self.NestMouseOver`) false false))

(event `HungerDescreaseChick1`
  (bind _chick1hunger (`self.Chick1Hunger`))
  ; Chick 1 Hunger
  (`KismetSystemLibrary.Delay` (+ (- (`self.ChickHungerTime`) (* (`self.Chick1FedAmt`) -1)) (`KismetMathLibrary.RandomFloatInRange` -3.0 3.0)) :!label _label)
  (if (< _chick1hunger 0.01)
    (`SceneComponent.SetVisibility` (`self.Chick1`) false false :!label _label_2)
    (`KismetSystemLibrary.PrintString` "Chick 1 Perished!")
    (bind _asui_hunger (cast `/Game/UI/UI_Hunger` (`self.UIHungerObject`)))
    (`/Game/UI/UI_Hunger.Chick1Perished` _asui_hunger)
    (elif (> _chick1hunger 0.0)
      (bind _output_get (set `self.Chick1Hunger` (`KismetMathLibrary.FClamp` (- (`self.Chick1Hunger`) 0.2))))
      (`KismetSystemLibrary.PrintString` (`KismetStringLibrary.BuildString_Double` "Chich Hunger Increased" "Chick 1 Satiation:" _output_get))
      (goto _label))))

(event `FeedChick1`
  ; Feed Chick 1
  (set `self.Chick1Hunger` (`KismetMathLibrary.FClamp` (+ (`self.Chick1Hunger`) 0.5)))
  (set `self.Chick1FedAmt` (+ (`self.Chick1FedAmt`) 1))
  (`GameplayStatics.PlaySound2D` "/Game/Audio/ruru_1.ruru_1" 0.3 2.0 0.0 null null))

(event `Chick2HungerDecrease`
  (bind _chick2hunger (`self.Chick2Hunger`))
  ; Chick 2 Hunger
  (`KismetSystemLibrary.Delay` (+ (- (`self.ChickHungerTime`) (* (`self.Chick2FedAmt`) -1)) (`KismetMathLibrary.RandomFloatInRange` -3.0 3.0)) :!label _label_3)
  (if (< _chick2hunger 0.01)
    (`SceneComponent.SetVisibility` (`self.Chick2`) false false :!label _label_4)
    (`KismetSystemLibrary.PrintString` "Chick 2 Perished!")
    (bind _asui_hunger (cast `/Game/UI/UI_Hunger` (`self.UIHungerObject`)))
    (`/Game/UI/UI_Hunger.Chick2Perished` _asui_hunger)
    (elif (> _chick2hunger 0.0)
      (bind _output_get (set `self.Chick2Hunger` (`KismetMathLibrary.FClamp` (- _chick2hunger 0.2))))
      (`KismetSystemLibrary.PrintString` (`KismetStringLibrary.BuildString_Double` "Chich Hunger Increased" "Chick 2 Satiation:" _output_get))
      (goto _label_3))))

(event `self.ReceiveTick`
  (params (DeltaSeconds :type "Float (single-precision)"))
  ; TICK
)

(event `FeedChick2`
  ; FeedChick2
  (set `self.Chick2Hunger` (`KismetMathLibrary.FClamp` (+ (`self.Chick2Hunger`) 0.5)))
  (set `self.Chick2FedAmt` (+ (`self.Chick2FedAmt`) 1))
  (`GameplayStatics.PlaySound2D` "/Game/Audio/ruru_1.ruru_1" 0.25 2.0 0.0 null null))

(event `Chick3HungerDescrease`
  (bind _chick3hunger (`self.Chick3Hunger`))
  ; Chick 3 Hunger
  (`KismetSystemLibrary.Delay` (+ (- (`self.ChickHungerTime`) (* (`self.Chick3FedAmt`) -1)) (`KismetMathLibrary.RandomFloatInRange` -3.0 3.0)) :!label _label_5)
  (if (< _chick3hunger 0.01)
    (`SceneComponent.SetVisibility` (`self.Chick3`) false false :!label _label_6)
    (`KismetSystemLibrary.PrintString` "Chick 3 Perished!")
    (bind _asui_hunger (cast `/Game/UI/UI_Hunger` (`self.UIHungerObject`)))
    (`/Game/UI/UI_Hunger.Chick3Perished` _asui_hunger)
    (elif (> _chick3hunger 0.0)
      (bind _output_get (set `self.Chick3Hunger` (`KismetMathLibrary.FClamp` (- _chick3hunger 0.2))))
      (`KismetSystemLibrary.PrintString` (`KismetStringLibrary.BuildString_Double` "Chich Hunger Increased" "Chick 3 Satiation:" _output_get))
      (goto _label_5))))

(event `FeedChick3`
  ; FeedChick3
  (set `self.Chick3Hunger` (`KismetMathLibrary.FClamp` (+ (`self.Chick3Hunger`) 0.5)))
  (set `self.Chick3FedAmt` (+ (`self.Chick3FedAmt`) 1))
  (`GameplayStatics.PlaySound2D` "/Game/Audio/ruru_1.ruru_1" 0.2 2.0 0.0 null null))

(event `self.ReceiveAnyDamage`
  (params (Damage :type "Float (single-precision)") (DamageType :type "DamageType Object Reference") (InstigatedBy :type "Controller Object Reference") (DamageCauser :type "Actor Object Reference"))
  (bind _returnvalue (`KismetMathLibrary.RandomIntegerInRange` 1 3))
  (`KismetSystemLibrary.PrintString` "NestDamaged")
  (if (== _returnvalue 1) :!label _label_7
    (`KismetSystemLibrary.PrintString` "DroneKilled C1")
    (goto _label_2)
    (elif (== _returnvalue 2)
      (`KismetSystemLibrary.PrintString` "DroneKilled C2")
      (goto _label_4)
      (elif (== 3 _returnvalue)
        (`KismetSystemLibrary.PrintString` "DroneKilled C3")
        (goto _label_6)))))

(event `OnTakeRadialDamage_Event`
  (params (DamagedActor :type "Actor Object Reference") (Damage :type "Float (single-precision)") (DamageType :type "DamageType Object Reference") (Origin :type "Vector Structure") (HitInfo :type "HitResult Structure (by ref)") (InstigatedBy :type "Controller Object Reference") (DamageCauser :type "Actor Object Reference"))
  (`KismetSystemLibrary.PrintString` "Nest DamangedR")
  (goto _label_7))

(fn `ShowTutorial`
  (if (not (`self.TutorialPlayed`))
    (bind _asbp_owl (cast `/Game/Owl/BP_Owl` (`GameplayStatics.GetPlayerPawn` 0)))
    (`/Game/Owl/BP_Owl.HideTutorial` _asbp_owl)
    (bind _returnvalue (`|CreateWidget` "/Game/UI/UI_Tutorial.UI_Tutorial_C" (`GameplayStatics.GetPlayerController` 0)))
    (`UserWidget.AddToViewport` _returnvalue 0)
    (set `self.TutorialUI` _returnvalue)
    (`UserWidget.PlayAnimation` _returnvalue (`/Game/UI/UI_Tutorial.FeedAnimation` _returnvalue) 0.0 1 "Forward" -0.1 false)
    (set `self.TutorialPlayed` true)
    (set `self.TutorialRemoved` false)))

(fn `UserConstructionScript`)