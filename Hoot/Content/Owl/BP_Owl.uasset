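; The owl actor flies on the X/Z plane, perches on buildings or its nest, hoots and dives for beetles.
; Tick uses state flags to switch pose visibility, interpolate movement and zoom the spring arm, with a Y offset while perched.
; Hooting alerts overlapping beetles, while dive overlaps eat them to refill hunger, which a delay loop drains.
; It also creates the hunger UI and plays tutorial animations on delays and landing.
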(event `self.ReceiveBeginPlay`
  ; Init
  (`SceneComponent.SetVisibility` (`self.Diving`) false false)
  (`SceneComponent.SetVisibility` (`self.Hooting`) false false)
  (`SceneComponent.SetVisibility` (`self.Perched`) false false)
  (`SceneComponent.SetVisibility` (`self.Flying`) false false)
  (set `self.TargetLocation` (`self.K2_GetActorLocation`))
  (set `self.OwlHunger` 0.5)
  (`self.HungerBarDecrease`)
  (bind _returnvalue (`|CreateWidget` "/Game/UI/UI_Hunger.UI_Hunger_C"))
  (set `self.HungerBarScreen` _returnvalue)
  (`UserWidget.AddToViewport` _returnvalue 900)
  (bind _output_get (set `/Game/UI/UI_Hunger.NestObject` (`self.NestObject`) _returnvalue))
  (bind _asbp_nest (cast `/Game/Owl/BP_Nest` _output_get)
    (:`then`
      (set `self.NestY` (- (.y (`SceneComponent.K2_GetComponentLocation` (`/Game/Owl/BP_Nest.Nest` _asbp_nest))) 1.0))
      (`self.NestTutorial`)
      (`self.PerchTutorial`)
      (`self.Hunger Tutorial`)
      (`self.BoostTutorial`))
    (:`CastFailed`
      (`KismetSystemLibrary.PrintString` "set nest object"))))

(event `NestTutorial`
  (`KismetSystemLibrary.Delay` 45.0)
  (bind _asui_tutorial (cast `/Game/UI/UI_Tutorial` (`self.TutorialUI`)))
  (`UserWidget.PlayAnimation` _asui_tutorial (`/Game/UI/UI_Tutorial.NestTutorial` _asui_tutorial) 0.0 1 "Forward" 0.7 false))

(event `OffSetPerchY`
  ; Owl State
  (if (not (`self.HasYOffSet`))
    (if (== (`self.PerchObject`) (`self.NestObject`))
      (`self.K2_SetActorLocation` (`KismetMathLibrary.MakeVector` (.x (`self.K2_GetActorLocation`)) (`self.NestY`) (.z (`self.K2_GetActorLocation`))))
      (else
        (`self.K2_SetActorLocation` (`KismetMathLibrary.MakeVector` (.x (`self.K2_GetActorLocation`)) (`self.TargetPerchY`) (.z (`self.K2_GetActorLocation`))))))
    (set `self.HasYOffSet` true)))

(event `self.ReceiveTick`
  (params (DeltaSeconds :type "Float (single-precision)"))
  (bind _isdiving (`self.isDiving`))
  (bind _perched (`self.Perched`))
  (bind (_returnvalue_x _returnvalue_y _returnvalue_z) (`KismetMathLibrary.BreakVector` (`KismetMathLibrary.VInterpTo` (`self.K2_GetActorLocation`) (`self.PerchTarget`) DeltaSeconds (* (`self.MovementSpeed`) 5.0))))
  (bind (_returnvalue_x_2 _returnvalue_y_2 _returnvalue_z_2) (`KismetMathLibrary.BreakVector` (`KismetMathLibrary.VInterpTo` (`self.K2_GetActorLocation`) (`self.TargetLocation`) (`GameplayStatics.GetWorldDeltaSeconds`) (`KismetMathLibrary.FClamp` (* (`self.MovementSpeed`) 1.0) 1.0 2.0))))
  ; Owl State
  ;; Perching?
  (if (`self.IsPerched`)
    (bind _ashoot_player_controller (cast `/Game/Owl/Hoot_PlayerController` (`GameplayStatics.GetPlayerController` 0)))
    (set `/Game/Owl/Hoot_PlayerController.IsPerching` true _ashoot_player_controller)
    (`SceneComponent.SetVisibility` _perched true false)
    ; Perch Camera
    (`self.OffSetPerchY`)
    (bind _ashoot_player_controller_2 (cast `/Game/Owl/Hoot_PlayerController` (`GameplayStatics.GetPlayerController` 0)))
    (if (== (`self.PerchObject`) (`self.NestObject`))
      ; On Nest
      (set `SpringArmComponent.TargetArmLength` (`KismetMathLibrary.FInterpTo` (`SpringArmComponent.TargetArmLength` (`self.SpringArm`)) 450.0 DeltaSeconds 8.0) (`self.SpringArm`))
      (bind _asui_tutorial (cast `/Game/UI/UI_Tutorial` (`self.TutorialUI`)))
      (`UserWidget.PlayAnimation` _asui_tutorial null 0.0 1 "Forward" 1.0 false)
      (bind _asbp_nest (cast `/Game/Owl/BP_Nest` (`self.NestObject`)))
      (`/Game/Owl/BP_Nest.ShowTutorial` _asbp_nest)
      (else
        ; On SpawnedBuilding
        (set `SpringArmComponent.TargetArmLength` (`KismetMathLibrary.FInterpTo` (`SpringArmComponent.TargetArmLength` (`self.SpringArm`)) (`/Game/Owl/Hoot_PlayerController.LastPerchedZoom` _ashoot_player_controller_2) DeltaSeconds 5.0) (`self.SpringArm`))))
    (else
      (`SceneComponent.SetVisibility` (`self.Flying`) true false)
      (`SceneComponent.SetVisibility` _perched false false)
      (`SceneComponent.SetVisibility` (`self.Hooting`) false false)
      ;; Landing?
      (if (`self.IsLanding`)
        ; Landing
        (`self.K2_SetActorLocation` (`KismetMathLibrary.MakeVector` _returnvalue_x (+ _returnvalue_y 0.01) _returnvalue_z))
        (if (== (`self.PerchTarget`) (`SceneComponent.K2_GetComponentLocation` (`self.Root/Collision`)) :`ErrorTolerance` 20.0)
          (`KismetSystemLibrary.PrintString` "Owl Landed")
          (`self.ShowTutorial`)
          (set `self.IsLanding` false)
          ; Diving for Critters
          (set `self.IsPerched` true)
          (`SceneComponent.SetVisibility` (`self.Flying`) false false))
        (else
          ;; Diving?
          (if _isdiving
            (`SceneComponent.SetVisibility` (`self.Flying`) false false)
            (`SceneComponent.SetVisibility` (`self.Diving`) true false)
            (`self.K2_SetActorLocation` (`KismetMathLibrary.MakeVector` (.x (`KismetMathLibrary.VInterpTo` (`self.K2_GetActorLocation`) (`self.CritterTarget`) DeltaSeconds (* (`self.MovementSpeed`) (`self.CritterDiveSpeedMultiplier`)))) 0.0 (.z (`KismetMathLibrary.VInterpTo` (`self.K2_GetActorLocation`) (`self.CritterTarget`) DeltaSeconds (* (`self.MovementSpeed`) (`self.CritterDiveSpeedMultiplier`))))) true)
            (`KismetSystemLibrary.Delay` 2.0)
            (set `self.isDiving` false)
            (elif (`KismetMathLibrary.BooleanNOR` _isdiving (`self.IsPerched`))
              ; FLYING
              (`self.HideTutorial`)
              (`SceneComponent.SetVisibility` (`self.Flying`) true false)
              (`SceneComponent.SetVisibility` (`self.Diving`) false false)
              (if (< (`KismetMathLibrary.Distance2D` (`KismetMathLibrary.Conv_VectorToVector2D` (`self.TargetLocation`)) (`KismetMathLibrary.Conv_VectorToVector2D` (`self.K2_GetActorLocation`))) 15.0)
                (set `self.bIsMoving` false)
                (else
                  (set `self.bIsMoving` true)
                  (`self.K2_SetActorLocation` (`KismetMathLibrary.MakeVector` _returnvalue_x_2 0.0 _returnvalue_z_2) true)
                  (if (`self.isTossing`)
                    (set `SpringArmComponent.TargetArmLength` (`KismetMathLibrary.FInterpTo` (`SpringArmComponent.TargetArmLength` (`self.SpringArm`)) 3200.0 DeltaSeconds 0.6) (`self.SpringArm`))
                    (else
                      ; fly Cam
                      (set `SpringArmComponent.TargetArmLength` (`KismetMathLibrary.FInterpTo` (`SpringArmComponent.TargetArmLength` (`self.SpringArm`)) 1500.0 DeltaSeconds 1.0) (`self.SpringArm`))
                      (`SceneComponent.K2_AddWorldOffset` (`self.SpringArm`) (0.0 0.0 0.0) false false))))))))))))

(event `ResetY`
  ; Owl State
  (`self.K2_SetActorLocation` (`KismetMathLibrary.MakeVector` (.x (`self.K2_GetActorLocation`)) 0.0 (.z (`self.K2_GetActorLocation`))))
  (set `self.HasYOffSet` false))

(event `PerchTutorial`
  (`KismetSystemLibrary.Delay` 5.0)
  (bind _asui_tutorial (cast `/Game/UI/UI_Tutorial` (`self.TutorialUI`)))
  (`UserWidget.PlayAnimation` _asui_tutorial (`/Game/UI/UI_Tutorial.PerchTutorial` _asui_tutorial) 0.0 1 "Forward" 0.7 false))

(event `Hunger Tutorial`
  (`KismetSystemLibrary.Delay` 25.0)
  (bind _asui_tutorial (cast `/Game/UI/UI_Tutorial` (`self.TutorialUI`)))
  (`UserWidget.PlayAnimation` _asui_tutorial (`/Game/UI/UI_Tutorial.HungerTutorial` _asui_tutorial) 0.0 1 "Forward" 0.4 false))

(event `TossCamera`
  (params (TossCameraDistance :type "Float (double-precision)"))
  (set `self.isTossing` true))

(event `Hoot`
  (bind _hooting (`self.Hooting`))
  (bind _perched (`self.Perched`))
  ; Perch And Hoot
  (set `PrimitiveComponent.bGenerateOverlapEvents` true (`self.HootSphere`))
  (`KismetSystemLibrary.PrintString` "HOOT")
  (`GameplayStatics.PlaySound2D` "/Game/Audio/ruru_1.ruru_1" 0.14 1.0 0.0 null null)
  (`SceneComponent.SetVisibility` _hooting true false)
  (`SceneComponent.SetVisibility` _perched false false)
  (`KismetSystemLibrary.Delay` 1.0)
  (`SceneComponent.SetVisibility` _hooting false false)
  (`SceneComponent.SetVisibility` _perched true false)
  ; HootAtBeetles
  (bind _filteredarray (`KismetArrayLibrary.FilterArray` (`PrimitiveComponent.GetOverlappingActors` (`self.HootSphere`) null) "/Game/Blueprints/Critters/BP_Beetle.BP_Beetle_C"))
  (for (_ _array_index) _filteredarray
    (bind _output (`|GetArrayItem` _filteredarray _array_index))
    (`KismetSystemLibrary.PrintString` (`KismetStringLibrary.BuildString_Object` "" "Hoot heard by:" _output))
    (bind _asbp_beetle (cast `/Game/Blueprints/Critters/BP_Beetle` _output))
    (`/Game/Blueprints/Critters/BP_Beetle.HootHeard` _asbp_beetle)
    (`KismetSystemLibrary.PrintString` "Bug Checked")
    (set `PrimitiveComponent.bGenerateOverlapEvents` false (`self.HootSphere`))))

(event `BoostTutorial`
  (`KismetSystemLibrary.Delay` 65.0)
  (bind _asui_tutorial (cast `/Game/UI/UI_Tutorial` (`self.TutorialUI`)))
  (`UserWidget.PlayAnimation` _asui_tutorial (`/Game/UI/UI_Tutorial.BoostTutorial` _asui_tutorial) 0.0 1 "Forward" 0.4 false))

(event `HungerBarDecrease`
  ; Hunger
  (if (== (`self.OwlHunger`) 0.0)
    (`self.K2_DestroyActor`)
    (elif (> (`self.OwlHunger`) 0.0)
      (bind _output_get (set `self.OwlHunger` (`KismetMathLibrary.FClamp` (- (`self.OwlHunger`) 0.05)) :!label _label))
      (`KismetSystemLibrary.PrintString` (`KismetStringLibrary.BuildString_Double` "Hunger Increased" "Owl Satiation:" _output_get))
      (`KismetSystemLibrary.Delay` (`self.HungerTime`))
      (goto _label))))

(event `self.Box.OnComponentBeginOverlap`
  (params (OverlappedComponent :type "PrimitiveComponent Object Reference") (OtherActor :type "Actor Object Reference") (OtherComp :type "PrimitiveComponent Object Reference") (OtherBodyIndex :type Integer) (bFromSweep :type Boolean) (SweepResult :type "HitResult Structure (by ref)"))
  ; CatchCritter
  (if (and (`self.isDiving`) (`self.ActorHasTag` OtherActor "critter"))
    (`KismetSystemLibrary.PrintString` (`KismetStringLibrary.BuildString_Object` "" "Hit Critter: " OtherActor))
    (bind _asbp_beetle (cast `/Game/Blueprints/Critters/BP_Beetle` OtherActor)
      (:`then`
        (`/Game/Blueprints/Critters/BP_Beetle.EatMe` _asbp_beetle)
        (`GameplayStatics.PlaySound2D` "/Game/Blueprints/Critters/119816__cmusounddesign__jbf-squirrel-run.119816__cmusounddesign__jbf-squirrel-run" 0.2 1.6 0.0 null null)
        (`self.Eat`))
      (:`CastFailed`
        (`KismetSystemLibrary.PrintString` "Cast to Beetle Failed")))))

(event `Eat`
  (bind _owlhunger (`self.OwlHunger`))
  (bind _returnvalue (`KismetMathLibrary.FClamp` (+ 0.2 _owlhunger)))
  ; Hunger
  ;; EAT
  (if (< _owlhunger 100.0)
    (set `self.OwlHunger` _returnvalue)
    (`KismetSystemLibrary.PrintString` (`KismetStringLibrary.BuildString_Double` "Critter Eaten. \n " "Owl Satiation:" _returnvalue))
    (set `self.isDiving` false)))

(fn `HideTutorial`
  (if (not (`self.TutorialRemoved`))
    (bind _asui_tutorial (cast `/Game/UI/UI_Tutorial` (`self.TutorialUI`)))
    (`UserWidget.PlayAnimationReverse` _asui_tutorial (`/Game/UI/UI_Tutorial.HootTutorial` _asui_tutorial) 1.0 false)
    (bind _asui_tutorial_button_overlay (cast `/Game/UI/UI_TutorialButtonOverlay` (`self.UI_ButtonOverlayObject`)))
    (`UserWidget.PlayAnimationReverse` _asui_tutorial_button_overlay (`/Game/UI/UI_TutorialButtonOverlay.HootTutorial` _asui_tutorial_button_overlay) 1.0 false)
    (set `self.TutorialRemoved` true)
    (set `self.TutorialPlayed` false)))

(fn `SendCameraZoom`
  (bind _ashoot_player_controller (cast `/Game/Owl/Hoot_PlayerController` (`GameplayStatics.GetPlayerController` 0)))
  (set `/Game/Owl/Hoot_PlayerController.CameraZoom` (`SpringArmComponent.TargetArmLength` (`self.SpringArm`)) _ashoot_player_controller))

(fn `ShowTutorial`
  (bind _returnvalue (`|CreateWidget` "/Game/UI/UI_TutorialButtonOverlay.UI_TutorialButtonOverlay_C"))
  (`UserWidget.AddToViewport` _returnvalue 0)
  (`UserWidget.PlayAnimation` _returnvalue (`/Game/UI/UI_TutorialButtonOverlay.HootTutorial` _returnvalue) 0.0 1 "Forward" 1.0 false)
  (set `self.UI_ButtonOverlayObject` _returnvalue)
  (if (not (`self.TutorialPlayed`))
    (bind _returnvalue_2 (`|CreateWidget` "/Game/UI/UI_Tutorial.UI_Tutorial_C" (`GameplayStatics.GetPlayerController` 0)))
    (`UserWidget.AddToViewport` _returnvalue_2 0)
    (set `self.TutorialUI` _returnvalue_2)
    (`UserWidget.PlayAnimation` _returnvalue_2 (`/Game/UI/UI_Tutorial.HootTutorial` _returnvalue_2) 0.0 1 "Forward" 1.0 false)
    (set `self.TutorialPlayed` true)
    (set `self.TutorialRemoved` false)))

(fn `UserConstructionScript`)