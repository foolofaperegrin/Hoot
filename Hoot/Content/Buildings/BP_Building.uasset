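; BP_Building is a destructible building actor that takes damage until it is destroyed.
; AnyDamage subtracts incoming damage from Health, printing the remaining value, or destroys the actor and prints a message once Health reaches zero or below.
; The Destroyed event spawns a P_Smoke particle emitter using the actor's location, rotation and scale.
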(event `self.ReceiveAnyDamage`
  (params (Damage :type "Float (single-precision)") (DamageType :type "DamageType Object Reference") (InstigatedBy :type "Controller Object Reference") (DamageCauser :type "Actor Object Reference"))
  (bind _output_get (set `self.Health` (- (`self.Health`) Damage)))
  (if (<= (`self.Health`) 0.0)
    (`self.K2_DestroyActor`)
    (`KismetSystemLibrary.PrintString` "Building Destroyed")
    (else
      (`KismetSystemLibrary.PrintString` (`KismetStringLibrary.BuildString_Double` "Damage to Building:" "" _output_get)))))

(event `self.ReceiveDestroyed`
  (`GameplayStatics.SpawnEmitterAtLocation` "/Game/StarterContent/Particles/P_Smoke.P_Smoke" (.location (`self.GetTransform`)) (.rotation (`self.GetTransform`)) (.scale (`self.GetTransform`))))

(fn `UserConstructionScript`)