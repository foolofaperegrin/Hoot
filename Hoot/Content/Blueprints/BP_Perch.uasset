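; BP_Perch is a clickable, destructible tree perch where the player's owl can land.
; Clicking it flags an unperched BP_Owl as landing and sets its PerchTarget from capsule markers at Y=0.
; X and Z use separate random picks, which can mix capsules and never select the fourth.
; Any damage removes one Health, destroying the actor at zero, while any actor overlap resets Health.
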(event `OnTakeRadialDamage_Event` :!signature `self.OnTakeRadialDamage`
  (params (DamagedActor :type "Actor Object Reference") (Damage :type "Float (single-precision)") (DamageType :type "DamageType Object Reference") (Origin :type "Vector Structure") (HitInfo :type "HitResult Structure (by ref)") (InstigatedBy :type "Controller Object Reference") (DamageCauser :type "Actor Object Reference"))
  (add `self.OnTakeRadialDamage` (delegate `OnTakeRadialDamage_Event`)))

(event `self.ReceiveBeginPlay`
  (`PrimitiveComponent.SetTranslucentSortPriority` (`self.PerchSprite`) -1)
  (`self.EnableInput` (`GameplayStatics.GetPlayerController` 0)))

(event `self.ReceiveAnyDamage`
  (params (Damage :type "Float (single-precision)") (DamageType :type "DamageType Object Reference") (InstigatedBy :type "Controller Object Reference") (DamageCauser :type "Actor Object Reference"))
  (bind _output_get (set `self.Health` (- (`self.Health`) 1.0)))
  (`KismetSystemLibrary.PrintString` "tree damaged")
  (if (== _output_get 0.0)
    (`self.K2_DestroyActor`)))

(event `self.ReceiveActorBeginOverlap`
  (params (OtherActor :type "Actor Object Reference"))
  (set `self.Health` 25.0))

(event `self.ReceiveActorOnClicked`
  (params (ButtonPressed :type "Key Structure"))
  (`KismetSystemLibrary.PrintString` "Perch Clicked")
  (bind _asbp_owl (cast `/Game/Owl/BP_Owl` (`GameplayStatics.GetPlayerPawn` 0)))
  (if (not (`/Game/Owl/BP_Owl.IsPerched` _asbp_owl))
    (set `/Game/Owl/BP_Owl.IsLanding` true _asbp_owl)
    (`KismetSystemLibrary.PrintString` "Owl is Landing")
    (set `/Game/Owl/BP_Owl.PerchTarget` (`KismetMathLibrary.MakeVector` (.x (`SceneComponent.K2_GetComponentLocation` (`|GetArrayItem` (`|MakeArray` (`self.Capsule`) (`self.Capsule1`) (`self.Capsule2`) (`self.Capsule3`)) (`KismetMathLibrary.RandomInteger` 3)))) 0.0 (.z (`SceneComponent.K2_GetComponentLocation` (`|GetArrayItem` (`|MakeArray` (`self.Capsule`) (`self.Capsule1`) (`self.Capsule2`) (`self.Capsule3`)) (`KismetMathLibrary.RandomInteger` 3))))) _asbp_owl)))

(event `self.Capsule.OnClicked`
  (params (TouchedComponent :type "PrimitiveComponent Object Reference") (ButtonPressed :type "Key Structure")))

(event `self.Capsule1.OnClicked`
  (params (TouchedComponent :type "PrimitiveComponent Object Reference") (ButtonPressed :type "Key Structure")))

(fn `UserConstructionScript`)