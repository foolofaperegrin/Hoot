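; BP_Owl is a Paper2D owl actor that shows its flipbook, hides its static sprite at start, and glides toward TargetLocation.
; Tick applies VInterpTo to X and Z with sweep, leaving Y unwired, at MovementSpeed scaled by delta time.
; The arrival check tests distance below zero, so it never passes and IsMoving is always set true.
; Capsule hits only print a debug message.
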(event `self.ReceiveBeginPlay`
  (`SceneComponent.SetVisibility` (`self.PaperSprite`) false false)
  (`SceneComponent.SetVisibility` (`self.PaperFlipbook`) true false))

(event `self.ReceiveTick`
  (params (DeltaSeconds :type "Float (single-precision)"))
  (bind (_returnvalue_x _returnvalue_y _returnvalue_z) (`KismetMathLibrary.BreakVector` (`KismetMathLibrary.VInterpTo` (`self.K2_GetActorLocation`) (`self.TargetLocation`) DeltaSeconds (* (`self.MovementSpeed`) DeltaSeconds))))
  (bind _returnvalue (`KismetMathLibrary.Distance2D` (`KismetMathLibrary.Conv_VectorToVector2D` (`self.TargetLocation`)) (`KismetMathLibrary.Conv_VectorToVector2D` (`self.K2_GetActorLocation`))))
  (if (< _returnvalue 0.0)
    (`KismetSystemLibrary.PrintString` (`KismetStringLibrary.BuildString_Double` "DISTANCE =")))
  (if (< _returnvalue 0.0)
    (set `self.bIsMoving` false)
    (else
      (set `self.bIsMoving` true)
      (`self.K2_SetActorLocation` (`KismetMathLibrary.MakeVector` _returnvalue_x 0.0 _returnvalue_z) true))))

(event `self.Capsule.OnComponentHit`
  (params (HitComponent :type "PrimitiveComponent Object Reference") (OtherActor :type "Actor Object Reference") (OtherComp :type "PrimitiveComponent Object Reference") (NormalImpulse :type "Vector Structure") (Hit :type "HitResult Structure (by ref)"))
  (`KismetSystemLibrary.PrintString` "Owl Collided with something"))

(fn `UserConstructionScript`)